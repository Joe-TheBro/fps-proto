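; Game instance that drives menu flow, multiplayer session hosting and joining, and network/travel error handling.
; Menu events mostly lazily create and cache widgets, and a save-slot check opens the main menu or, without a save, options.
; LaunchLobby creates a session and opens Lobby as a listen server; JoinServer joins a given search result.
; Failures route to DisplayErrorMessage, which is an empty stub, as are the error-to-string converters.
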(event `SaveGameCheck`
  ;[1 1 1] Save
  (bind _returnvalue (`GameplayStatics.DoesSaveGameExist` (`self.PlayerSettingsSave`)))
  (if _returnvalue
    (`self.Show Main Menu`)
    (set `self.CreatedSaveFile` true)
    (else
      (`self.ShowOptionsMenu`)
      (set `PlayerController.bShowMouseCursor` false (`GameplayStatics.GetPlayerController` 0)))))

(event `self.HandleNetworkError`
  (params (FailureType :type "ENetworkFailure Enum" :default "NetDriverAlreadyExists") (bIsServer :type Boolean))
  ;[1 1 1] Handle Network Errors and fis messafe
  (if bIsServer
    _
    (else
      _))
  (`self.DisplayErrorMessage` (`self.NetErrorToString` FailureType)))

(event `Show Play Menu`
  (bind _returnvalue (`GameplayStatics.GetPlayerController` 0))
  ;[1 1 1] Show Play Menu
  (`/Engine/EditorBlueprintResources/StandardMacros.IsValid` (`self.PlayMenuWB`)
    (:`Is Valid`
      _)
    (:`Is Not Valid`
      (bind _returnvalue_2 (`|CreateWidget` "/Game/Blueprints/UI/MainMenu/PlayMenu.PlayMenu_C" _returnvalue))
      (set `self.PlayMenuWB` _returnvalue_2)))
  (`UserWidget.AddToViewport` (`self.PlayMenuWB`) 0)
  (set `PlayerController.bShowMouseCursor` true _returnvalue))

(event `Show Main Menu`
  (bind _returnvalue (`GameplayStatics.GetPlayerController` 0))
  ;[1 1 1] Show Main Menu
  (`/Engine/EditorBlueprintResources/StandardMacros.IsValid` (`self.MainMenuWB`)
    (:`Is Valid`
      _)
    (:`Is Not Valid`
      (bind _returnvalue_2 (`|CreateWidget` "/Game/Blueprints/UI/MainMenu/MainMenu.MainMenu_C" _returnvalue))
      (set `self.MainMenuWB` _returnvalue_2)))
  (`UserWidget.AddToViewport` (`self.MainMenuWB`) 0)
  (set `PlayerController.bShowMouseCursor` true _returnvalue))

(event `ShowLoadingScreen`
  ;[1 1 1] Shows loading screen when called.
  (`/Engine/EditorBlueprintResources/StandardMacros.IsValid` (`self.LoadingScreenWB`)
    (:`Is Valid`
      (`UserWidget.AddToViewport` (`self.LoadingScreenWB`) 0))
    (:`Is Not Valid`
      (bind _returnvalue (`|CreateWidget` "/Game/Blueprints/UI/AllLevels/LoadingScreen.LoadingScreen_C" (`GameplayStatics.GetPlayerController` 0)))
      (set `self.LoadingScreenWB` _returnvalue))))

(event `self.HandleTravelError`
  (params (FailureType :type "ETravelFailure Enum" :default "NoLevel"))
  ;[1 1 1] Handle Travel errors and dis message
  (`self.DisplayErrorMessage` (`self.TravelToString` FailureType)))

(event `DestroySessionCaller`
  (params (`Player Controller` :type "PlayerController Object Reference"))
  ;[1 1 1] DEstroy Session WHen Called
  (`DestroySessionCallbackProxy.DestroySession` `Player Controller`))

(event `LaunchLobby`
  (params (NumberOfPlayers :type Integer) (`EnableLan?` :type Boolean) (ServerName :type Text))
  ;[1 1 1] Launch lobby with settings
  (set `self.MaxPlayers` NumberOfPlayers)
  (set `self.ServerName` ServerName)
  (`self.ShowLoadingScreen`)
  (`CreateSessionCallbackProxy.CreateSession` (`GameplayStatics.GetPlayerController` 0) (`self.MaxPlayers`) `EnableLan?`
    (:`OnSuccess`
      (`GameplayStatics.OpenLevel` "Lobby" true "listen"))
    (:`OnFailure`
      (`self.DisplayErrorMessage` "Failed To Create Session Please Try Again."))))

(event `ShowHostMenu`
  ;[1 1 1] Host Game Menu
  (`/Engine/EditorBlueprintResources/StandardMacros.IsValid` (`self.HostMenuWB`)
    (:`Is Valid`
      _)
    (:`Is Not Valid`
      (bind _returnvalue (`|CreateWidget` "/Game/Blueprints/UI/MainMenu/HostMenu.HostMenu_C" (`GameplayStatics.GetPlayerController` 0)))
      (set `self.HostMenuWB` _returnvalue)))
  (`UserWidget.AddToViewport` (`self.HostMenuWB`) 0))

(event `JoinServer`
  (params (`Session To Join` :type "BlueprintSessionResult Structure"))
  ;[1 1 1] Join Server
  (`self.ShowLoadingScreen`)
  (`JoinSessionCallbackProxy.JoinSession` (`GameplayStatics.GetPlayerController` 0) `Session To Join`
    (:`OnFailure`
      (`self.DisplayErrorMessage` "Failed To Join Session Please Try Again."))))

(event `ShowServerMenu`
  ;[1 1 1] Shows server menu create each time its called
  (bind _returnvalue (`|CreateWidget` "/Game/Blueprints/UI/MainMenu/ServerMenu.ServerMenu_C" (`GameplayStatics.GetPlayerController` 0)))
  (`UserWidget.AddToViewport` _returnvalue 0))

(event `ShowOptionsMenu`
  ;[1 1 1] Show the options menu
  (`/Engine/EditorBlueprintResources/StandardMacros.IsValid` (`self.OptionsMenuWB`)
    (:`Is Valid`
      _)
    (:`Is Not Valid`
      (bind _returnvalue (`|CreateWidget` "/Game/Blueprints/UI/MainMenu/OptionsMenu.OptionsMenu_C" (`GameplayStatics.GetPlayerController` 0)))
      (set `self.OptionsMenuWB` _returnvalue)))
  (`UserWidget.AddToViewport` (`self.OptionsMenuWB`) 0))

(fn `NetErrorToString`
  (params (`Faliure type` :type "ENetworkFailure Enum" :default "NetDriverAlreadyExists"))
  (returns (Outstring :type String))
  (return ""))

(fn `TravelToString`
  (params (`Failure type` :type "ETravelFailure Enum" :default "NoLevel"))
  (returns (`Out String` :type String))
  (return ""))